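; Drivable Fabia car pawn that maps player input to throttle, steering and handbrake on its vehicle movement component.
; If the car is moving when the handbrake is pressed, a Delay loop rapidly spawns FabiaTMark actors at left and right tyre points until release, without rechecking speed.
; The camera arm takes the mesh's relative rotation on BeginPlay, then follows look input, with zoom limited to a fixed arm-length range.
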(event EventBeginPlay
  (Transformation|SetRelativeRotation (Variables|Default|GetCamArm) (Variables|/Script/Engine.SceneComponent|GetRelativeRotation (Variables|Character|GetMesh)) false false))

(event Input|ActionEvents|InputActionHandbrake
  (params (Key :type Key%20Structure))
  (bind _returnvalue (Transformation|GetActorRotation))
  (:Pressed
    (Variables|Default|SetHandbrake true)
    (Class|WheeledVehicleMovementComponent|SetHandbrakeInput (Variables|Default|GetVehicleMovement) (Variables|Default|GetHandbrake) :!label _label)
    (if (not (== (Class|WheeledVehicleMovementComponent|GetForwardSpeed (Variables|Default|GetVehicleMovement)) 0.0))
      (Game|SpawnActorfromClass "/Game/Fabia/FabiaTMark.FabiaTMark_C" (Math|Transform|MakeTransform (Transformation|GetWorldLocation (Variables|Default|GetTyremark_L)) _returnvalue "0.200000,0.200000,0.200000") "Undefined" 0 0 :!label _label_2)
      (Game|SpawnActorfromClass "/Game/Fabia/FabiaTMark.FabiaTMark_C" (Math|Transform|MakeTransform (Transformation|GetWorldLocation (Variables|Default|GetTyremark_R)) _returnvalue "0.200000,0.200000,0.200000") "Undefined" 0 0)
      (Utilities|FlowControl|Delay 0.01)
      (if (Variables|Default|GetHandbrake)
        (goto _label_2))))
  (:Released
    (Variables|Default|SetHandbrake false)
    (goto _label)))

(event Input|AxisEvents|InputAxisAccelerate/Reverse
  (params (AxisValue :type Float%20%28single-precision%29))
  (Class|WheeledVehicleMovementComponent|SetThrottleInput (Variables|Default|GetVehicleMovement) AxisValue))

(event Input|AxisEvents|InputAxisVehicleTurn
  (params (AxisValue :type Float%20%28single-precision%29))
  (Class|WheeledVehicleMovementComponent|SetSteeringInput (Variables|Default|GetVehicleMovement) AxisValue))

(event Input|AxisEvents|InputAxisCamX
  (params (AxisValue :type Float%20%28single-precision%29))
  (Transformation|AddRelativeRotation (Variables|Default|GetCamArm) (Math|Rotator|MakeRotator 0.0 0.0 AxisValue) false false))

(event Input|AxisEvents|InputAxisCamY
  (params (AxisValue :type Float%20%28single-precision%29))
  (Transformation|AddRelativeRotation (Variables|Default|GetCamArm) (Math|Rotator|MakeRotator 0.0 AxisValue 0.0) false false))

(event Input|AxisEvents|InputAxisCamZoom
  (params (AxisValue :type Float%20%28single-precision%29))
  (bind _camarm (Variables|Default|GetCamArm))
  (if (Math|Float|InRange(Float) (+ (* AxisValue -75.0) (Variables|/Script/Engine.SpringArmComponent|GetTargetArmLength _camarm)) 2.5e+02 1e+03)
    (Variables|/Script/Engine.SpringArmComponent|SetTargetArmLength _camarm (+ (* AxisValue -75.0) (Variables|/Script/Engine.SpringArmComponent|GetTargetArmLength _camarm)))))

(fn ConstructionScript)